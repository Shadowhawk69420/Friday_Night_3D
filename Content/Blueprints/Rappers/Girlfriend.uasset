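; Girlfriend is a child rapper Blueprint that adds an animated Speakers skeletal mesh to the behavior it inherits from its parent.
; On BeginPlay it starts the speaker idle montage once at an offset of the inherited animation rate, then scales that rate down as a rough tempo-matching fix.
; IdleAnim and the construction script only call their parent versions.
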(event EventBeginPlay
  (|CallParentFunction)
  (Utilities|FlowControl|DoOnce false
    (:Completed
      (Animation|Montage|PlayMontage (Variables|Default|GetSpeakers) "/Game/models/Characters/Girlfriend/Speaker_idle_anim_Speakers_Armature__Speakers_Montage.Speaker_idle_anim_Speakers_Armature__Speakers_Montage" (+ (Variables|Default|Getanimation_rate) 0.5)
        (:then
          ;[1 1 1] quick and easy fix to mach tempo_ very shit
          (Variables|Default|Setanimation_rate (/ (Variables|Default|Getanimation_rate) 1.2)))))))

(event EventIdleAnim
  (|CallParentFunction))

(fn ConstructionScript
  (|CallParentFunction))