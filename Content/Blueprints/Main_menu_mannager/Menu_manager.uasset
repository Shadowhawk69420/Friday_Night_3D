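; Menu manager Blueprint that sets up the main menu screen when play begins.
; It starts the FreakyMenu music, stores it in MenuMusic and shows the mouse cursor.
; It then reads LaunchedGame from the Funking_instance game instance: if true it adds the main menu and song fade-out widgets, otherwise the game creator credits widget.
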(event EventBeginPlay
  (bind _returnvalue (Audio|SpawnSound2D "/Game/Music/Menu_music/freakyMenu.freakyMenu" 1.0 1.0 0.0 0))
  (Variables|Default|Setmenu_music _returnvalue)
  (Variables|/Script/Engine.PlayerController|SetbShowMouseCursor (Game|GetPlayerController 0) true)
  (bind _asfunking_instance (Utilities|Casting|CastToFunking_instance (Game|GetGameInstance)))
  (if (Variables|/Game/Blueprints/Game_stuff/Funking_instance.Funking_instance_C|GetLaunched_game _asfunking_instance)
    (bind _returnvalue_2 (UserInterface|CreateWidget "/Game/Widgets/Menu_widgets/Main_menu.Main_menu_C"))
    (UserInterface|Viewport|AddtoViewport _returnvalue_2 0)
    (bind _returnvalue_3 (UserInterface|CreateWidget "/Game/Widgets/Gameplay_widgets/Fade_out_song.Fade_out_song_C"))
    (UserInterface|Viewport|AddtoViewport _returnvalue_3 0)
    (else
      (bind _returnvalue_4 (UserInterface|CreateWidget "/Game/Widgets/Menu_widgets/Credits_creator_of_game.Credits_creator_of_game_C"))
      (UserInterface|Viewport|AddtoViewport _returnvalue_4 0))))

(fn ConstructionScript)