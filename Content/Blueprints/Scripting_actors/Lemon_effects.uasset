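; Scripting actor for the Lemon effects: a dark vignette overlay plus a monster sequence that takes over the Mannager's arrows and health bar.
; Overwrite_arrows blocks enemy scoring, shows the demon vignette, then uses chained timers to switch arrow mode and lerp health from max to a target.
; A looping camera shake follows until Reset restores arrows and scoring, eases health to half max and clears the demon vignette.
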(event Custom|Toggle
  (params (Demon_vignete :type Boolean) (Vigente :type Boolean))
  (Default|ToggleVignete (Variables|Default|Getlemon_overlay_widget) Demon_vignete Vigente))

(event Custom|Overwrite_arrows
  ;[1 1 1] this sequence activates monster arroes and stuff
  (bind _outactors (Actor|GetAllActorsOfClass "/Game/Blueprints/Rythim_manger/Mannager.Mannager_C"))
  (Variables|Default|Setmannager_ref (Utilities|Array|Get(acopy) _outactors))
  (Variables|/Game/Blueprints/Rythim_manger/Mannager.Mannager_C|SetEnemy_can-score (Variables|Default|Getmannager_ref) false)
  (CallFunction|Toggle true true)
  (Variables|Default|SetCurrent_health (Variables|/Game/Blueprints/Rythim_manger/Mannager.Mannager_C|GetHealth (Variables|Default|Getmannager_ref)))
  (Utilities|Time|SetTimerbyEvent (delegate Custom|Event_health_to_max) 0.2))

(event Custom|Reset_to_full
  (bind _mannager_ref (Variables|Default|Getmannager_ref))
  (Variables|Default|SetCurrent_health (Variables|/Game/Blueprints/Rythim_manger/Mannager.Mannager_C|GetHealth (Variables|Default|Getmannager_ref)))
  (bind _alpha (Timeline|Timeline_0 PlayFromStart)
    (:Update
      (Variables|/Game/Blueprints/Rythim_manger/Mannager.Mannager_C|SetHealth _mannager_ref (Math|Float|Lerp (Variables|Default|GetCurrent_health) (/ (Variables|/Game/Blueprints/Rythim_manger/Mannager.Mannager_C|GetMax_health (Variables|Default|Getmannager_ref)) 2.0) _alpha))
      (Default|UpdateBar _mannager_ref))
    (:Finished
      (CallFunction|Toggle false true))))

(event Custom|Event_health_to_max
  ;[1 1 1] this sequence activates monster arroes and stuff
  (Variables|/Game/Blueprints/Rythim_manger/Mannager.Mannager_C|SetArrow_action_overwrite (Variables|Default|Getmannager_ref) "NewEnumerator1")
  (Variables|Default|SetCurrent_health (Variables|/Game/Blueprints/Rythim_manger/Mannager.Mannager_C|GetMax_health (Variables|Default|Getmannager_ref)))
  (Utilities|Time|SetTimerbyEvent (delegate Custom|Event_toggle_arrows) 1.0))

(event Custom|Reset
  ;[1 1 1] Resets stuff back to normal
  (Variables|/Game/Blueprints/Rythim_manger/Mannager.Mannager_C|SetArrow_action_overwrite (Variables|Default|Getmannager_ref) "NewEnumerator0")
  (Variables|/Game/Blueprints/Rythim_manger/Mannager.Mannager_C|SetEnemy_can-score (Variables|Default|Getmannager_ref) true)
  (Utilities|Time|ClearandInvalidateTimerbyHandle (Variables|Default|Getshake_timer))
  (Utilities|Time|SetTimerbyEvent (delegate Custom|Reset_to_full) 0.1))

(event Custom|Active_shake
  ;[1 1 1] shake
  (Camera|PlayWorldCameraShake "/Game/Blueprints/Screen_shakes/Monster_cam_shake.Monster_cam_shake_C" (Transformation|GetWorldLocation (Variables|/Script/Engine.PlayerCameraManager|GetTransformComponent (Game|GetPlayerCameraManager 0))) 5e+01 5e+01 1.0 true))

(event Custom|Shake
  ;[1 1 1] shake
  (bind _returnvalue (Utilities|Time|SetTimerbyEvent (delegate Custom|Active_shake) 0.1 true))
  (Variables|Default|Setshake_timer _returnvalue))

(event Custom|Event_toggle_arrows
  (bind _mannager_ref (Variables|Default|Getmannager_ref))
  ;[1 1 1] this sequence activates monster arroes and stuff
  (bind _alpha (Timeline|Health_to_min PlayFromStart)
    (:Update
      (Variables|/Game/Blueprints/Rythim_manger/Mannager.Mannager_C|SetHealth _mannager_ref (Math|Float|Lerp (Variables|Default|GetCurrent_health) (Variables|Default|Gettarquet_health) _alpha))
      (Default|UpdateBar _mannager_ref))
    (:Finished
      (CallFunction|Shake))))

(event EventBeginPlay
  (bind _returnvalue (UserInterface|CreateWidget "/Game/Widgets/Gameplay_widgets/Effect_widgets/Lemon_Dark_overlay.Lemon_Dark_overlay_C" (Game|GetPlayerController 0)))
  (bind _output_get (Variables|Default|Setlemon_overlay_widget _returnvalue))
  (UserInterface|Viewport|AddtoPlayerScreen _output_get -9)
  (CallFunction|Toggle false true))

(fn ConstructionScript)