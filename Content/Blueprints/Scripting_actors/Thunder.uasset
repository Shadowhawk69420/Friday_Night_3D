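; Thunder actor that creates recurring random lightning strikes during a song, startling the Girlfriend characters.
; It starts when the first Mannager actor signals SongStarted, then chains non-looping timers with random delays.
; Each strike briefly shows a Plane as the flash, then hides it while playing the thunder sound and a scared montage on every Girlfriend.
; A further random delay precedes rescheduling, keeping the cycle running indefinitely.
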(event Custom|Reset_thunder
  (CallFunction|ThunderTimmerRandom))

(event Custom|Start_logic
  (Utilities|Time|SetTimerbyEvent (delegate Custom|Thunder) (Math|Random|RandomFloatinRange 1.0 4.0)))

(event Custom|Thunder_timmer_random
  (Utilities|Time|SetTimerbyEvent (delegate Custom|Thunder) (Math|Random|RandomFloatinRange 1.0 4.0)))

(event Custom|Thunder
  (Rendering|SetVisibility (Variables|Default|GetPlane) true false)
  (Utilities|Time|SetTimerbyEvent (delegate Custom|Thunder_hide) 0.2))

(event Custom|Thunder_hide
  (bind _outactors (Actor|GetAllActorsOfClass "/Game/Blueprints/Rappers/Girlfriend.Girlfriend_C"))
  (for _array_element _outactors
    (Default|PlayInstantCustomAnim _array_element "/Game/models/Characters/Girlfriend/animations/gf_scared_Montage.gf_scared_Montage"))
  (Rendering|SetVisibility (Variables|Default|GetPlane) false false)
  (Audio|PlaySound2D "/Game/sounds/Thunder_que.Thunder_que" 1.0 1.0 0.0 0 0)
  (Utilities|Time|SetTimerbyEvent (delegate Custom|Reset_thunder) (Math|Random|RandomFloatinRange 2.0 6.0)))

(event EventBeginPlay
  (bind _outactors (Actor|GetAllActorsOfClass "/Game/Blueprints/Rythim_manger/Mannager.Mannager_C"))
  (EventDispatchers|BindEventtoSongStarted (Utilities|Array|Get(acopy) _outactors) (delegate Custom|Start_logic)))

(fn ConstructionScript)