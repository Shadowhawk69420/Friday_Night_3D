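; Blueprint function set for menu navigation that moves the player's view between menu screens: free play, first week and what's new.
; Each function finds the Menu_manager actor with GetAllActorsOfClass and takes the first result.
; It then calls SetViewTargetWithBlend on player controller 0, targeting that manager's free play camera, first week camera or what's new camera.
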(fn ScrolltoFreeplayView
  (bind _outactors (Actor|GetAllActorsOfClass 0 "/Game/Blueprints/Main_menu_mannager/Menu_manager.Menu_manager_C"))
  (Game|Player|SetViewTargetwithBlend (Game|GetPlayerController 0) (Variables|/Game/Blueprints/Main_menu_mannager/Menu_manager.Menu_manager_C|GetFree_play_cam (Utilities|Array|Get(acopy) _outactors)) 0.0 "VTBlend_Linear" 0.0 false))

(fn ScrolltoFirstWeekView
  (bind _outactors (Actor|GetAllActorsOfClass 0 "/Game/Blueprints/Main_menu_mannager/Menu_manager.Menu_manager_C"))
  (Game|Player|SetViewTargetwithBlend (Game|GetPlayerController 0) (Utilities|Array|Get(acopy) (Variables|/Game/Blueprints/Main_menu_mannager/Menu_manager.Menu_manager_C|GetWeek_cameras (Utilities|Array|Get(acopy) _outactors))) 0.0 "VTBlend_Linear" 0.0 false))

(fn ScrolltoWhat'sNew
  (bind _outactors (Actor|GetAllActorsOfClass 0 "/Game/Blueprints/Main_menu_mannager/Menu_manager.Menu_manager_C"))
  (Game|Player|SetViewTargetwithBlend (Game|GetPlayerController 0) (Variables|/Game/Blueprints/Main_menu_mannager/Menu_manager.Menu_manager_C|GetWhat's_new_camera (Utilities|Array|Get(acopy) _outactors)) 0.0 "VTBlend_Linear" 0.0 false))